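; BP_KitchenDoor9 is an interactable kitchen door that slides open and closed when OnInteract fires.
; Each interaction prints and flips the IsClosedDoor flag, then plays or reverses the OpenDoor timeline.
; The timeline's alpha drives a lerp that offsets the mesh a short distance along negative world Y from the actor's location, so the slide ignores actor rotation.
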(event `self.OnInteract`
  (params (InteractingPawn :type "Pawn Object Reference"))
  (bind (_returnvalue_x _returnvalue_y _returnvalue_z) (`KismetMathLibrary.BreakVector` (`self.K2_GetActorLocation`)))
  (bind _iscloseddoor (`self.IsClosedDoor`))
  (`KismetSystemLibrary.PrintString` (`KismetStringLibrary.Conv_BoolToString` _iscloseddoor))
  (bind _output_get (set `self.IsClosedDoor` _iscloseddoor))
  (if _output_get
    (set `self.IsClosedDoor` false)
    (bind (_direction _dooralpha) (`Timeline|OpenDoor` :!label _label)
      (:`Update`
        (`SceneComponent.K2_SetWorldLocation` (`self.MeshComponent`) (`KismetMathLibrary.MakeVector` _returnvalue_x (+ (`KismetMathLibrary.Lerp` 0.0 -20.0 _dooralpha) _returnvalue_y) _returnvalue_z) false false)))
    (else
      (set `self.IsClosedDoor` true)
      (goto _label :!via `Reverse`))))

(fn `UserConstructionScript`)