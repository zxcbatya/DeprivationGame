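; Player character Blueprint with Enhanced Input movement, camera head bob and automatic depth of field.
; IA_Move moves the character along its forward and right vectors.
; While CinematicPlayable, toggled by PlayCinematic, is true, Tick starts walk or idle camera shakes based on velocity.
; A looping timer started on BeginPlay traces from the camera and sets post-process focal distance to the hit point.
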(event `PlayCinematic`
  (set `self.CinematicPlayable` (not (`self.CinematicPlayable`))))

(event `self.ReceiveTick`
  (params (DeltaSeconds :type "Float (single-precision)"))
  (if (`self.CinematicPlayable`)
    (`self.headblob`)))

(event `self.ReceiveBeginPlay`
  (`|ExecutionSequence`
    (:`then_0`
      (set `self.CharacterRef` self))
    (:`then_1`
      (`KismetSystemLibrary.K2_SetTimer` null "AutoDOF" 0.2 true))))

(event `EnhancedInput|/Game/BluePrints/Inputs/PayerIput/IA_Move`
  (params (ActionValue :type "Vector2D Structure") (ElapsedSeconds :type "Float (double-precision)") (TriggeredSeconds :type "Float (double-precision)") (InputAction :type "InputAction Object Reference" :default "/Game/BluePrints/Inputs/PayerIput/IA_Move.IA_Move"))
  (:`Triggered`
    (`self.AddMovementInput` (`self.GetActorForwardVector`) ActionValue_Y)))

(event `EnhancedInput|/Game/BluePrints/Inputs/PayerIput/IA_Move`
  (params (ActionValue :type "Vector2D Structure") (ElapsedSeconds :type "Float (double-precision)") (TriggeredSeconds :type "Float (double-precision)") (InputAction :type "InputAction Object Reference" :default "/Game/BluePrints/Inputs/PayerIput/IA_Move.IA_Move"))
  (:`Triggered`
    (`self.AddMovementInput` (`self.GetActorRightVector`) ActionValue_X)))

(event `AutoDOF`
  (bind _cameracomponent (`self.CameraComponent`))
  (bind _returnvalue (`SceneComponent.K2_GetComponentLocation` _cameracomponent))
  ; autoDof
  (bind (_outhit _returnvalue_2) (`KismetSystemLibrary.LineTraceSingle` _returnvalue (+ _returnvalue (* (`SceneComponent.GetForwardVector` _cameracomponent) 10000.0)) "TraceTypeQuery1"))
  (if _returnvalue_2
    (bind _output_get (set `self.focusLocation` (`KismetMathLibrary.VSize` (- (`.Location` (`GameplayStatics.BreakHitResult` _outhit)) (`SceneComponent.K2_GetComponentLocation` (`self.CameraComponent`))))))
    (set `CameraComponent.PostProcessSettings` (make `PostProcessSettings` :`DepthOfFieldFstop` 1.0 :`DepthOfFieldMinFstop` 11.0 :`DepthOfFieldFocalDistance` _output_get) (`self.CameraComponent`))))

(event `headblob`
  (bind _returnvalue (`GameplayStatics.GetPlayerController` 0))
  ; Headblob
  (if (> (`KismetMathLibrary.VSize` (`self.GetVelocity`)) 0.0)
    (`PlayerController.ClientStartCameraShake` :`self` _returnvalue :`Shake` "/Game/BluePrints/Player/CameraShakes/BP_CameraShakeWalk.BP_CameraShakeWalk_C")
    (else
      (`PlayerController.ClientStartCameraShake` :`self` _returnvalue :`Shake` "/Game/BluePrints/Player/CameraShakes/BP_CameraShakeIdle.BP_CameraShakeIdle_C"))))

(fn `UserConstructionScript`)