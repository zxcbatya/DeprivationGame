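; Game flow manager that sets up the player at level start and holds a currently disconnected intro sequence.
; BeginPlay caches the BP_Character pawn, waits briefly, then spawns a backpack at the pawn and has the character pick it up.
; IntroGame plays a cinematic, toggles input off and straight back on, and seats the character in a tagged vehicle.
; Its call, the intro monologue, black-screen creation and sound playback are all unwired.
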(event `self.ReceiveBeginPlay`
  (`self.CharacterRefFunction`)
  (`KismetSystemLibrary.Delay` 1.0)
  (bind _returnvalue (`|SpawnActorFromClass` "/Game/BluePrints/InteractableItems/BackPack/BP_BackPack.BP_BackPack_C" (`self.GetTransform` (`GameplayStatics.GetPlayerPawn` 0)) "Undefined" "MultiplyWithRoot" null null))
  (`BaseCharacter.PickUpItem` (`self.As BP Character`) _returnvalue))

(fn `CharacterRefFunction`
  (returns (`AsBP Character` :type "/Game/BluePrints/Player/BP_Character Object Reference"))
  (bind _asbp_character (cast `/Game/BluePrints/Player/BP_Character` (`GameplayStatics.GetPlayerPawn` 0))
    (:`then`
      (set `self.As BP Character` _asbp_character))
    (:`CastFailed`
      _))
  (return _asbp_character))

(fn `IntroGame`
  (`Widget.RemoveFromParent` (`self.BlackScreenWidget`))
  (bind _outactor (`LevelSequencePlayer.CreateLevelSequencePlayer` (`self.IntroCinematic`)))
  (`MovieSceneSequencePlayer.Play` (`LevelSequenceActor.SequencePlayer` _outactor))
  (`/Game/BluePrints/Player/BP_Character.PlayCinematic` (`self.As BP Character`))
  (`self.DisableInput` (`self.As BP Character`) (`GameplayStatics.GetPlayerController` 0))
  (`self.EnableInput` (`self.As BP Character`) (`GameplayStatics.GetPlayerController` 0))
  (`BaseCharacter.EnterVehicleByTag` (`self.As BP Character`) "Vehicle"))

(fn `UserConstructionScript`)