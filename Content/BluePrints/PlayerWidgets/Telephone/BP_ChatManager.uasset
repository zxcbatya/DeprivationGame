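; Chat manager for the in-game telephone, holding the AllChats array and exposing lookup, add-message, mark-read and get-all functions.
; GetChatByContactID linearly searches by contact ID, feeding both mutating functions.
; AddMessage reuses the last message's metadata, appends to CurrentChatMessages and updates only a local chat copy, ignoring BIsIncoming.
; MarkChatAsRead inserts a read-flagged copy at the found index instead of replacing the entry.
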(fn `AddMessage`
  (params (ContactID :type Name) (MessageText :type Text) (` bIsIncoming` :type Boolean))
  (returns (MessangeIndex :type Integer))
  (locals (LocalChat :type "/Game/BluePrints/PlayerWidgets/Telephone/data/S_ChatData Structure") (LocalMessange :type "/Game/BluePrints/PlayerWidgets/Telephone/data/S_MessageData Structure") (LocalIndex :type Integer :default 0) (CountUnread :type Text))
  (bind (_outchat _bfound) (`self.GetChatByContactID` ContactID))
  (if _bfound
    (for _array_element (`self.AllChats`)
      (if (== ContactID (break `/Game/BluePrints/PlayerWidgets/Telephone/data/S_ChatData` _array_element))
        (bind _output_get (set `local.LocalChat` _outchat))
        (set `local.LocalMessange` (make `/Game/BluePrints/PlayerWidgets/Telephone/data/S_MessageData` (break `/Game/BluePrints/PlayerWidgets/Telephone/data/S_MessageData` (`.LastMessage_12_F2B0695347BFB80FCB242B849E071437` (break `/Game/BluePrints/PlayerWidgets/Telephone/data/S_ChatData` _output_get))) (`.RecipientID_12_ADFBC22940C0FC30854926813C0F5B63` (break `/Game/BluePrints/PlayerWidgets/Telephone/data/S_MessageData` (`.LastMessage_12_F2B0695347BFB80FCB242B849E071437` (break `/Game/BluePrints/PlayerWidgets/Telephone/data/S_ChatData` _output_get)))) MessageText (`.Timestamp_14_474A67BA4F290977D851B184591D4D2A` (break `/Game/BluePrints/PlayerWidgets/Telephone/data/S_MessageData` (`.LastMessage_12_F2B0695347BFB80FCB242B849E071437` (break `/Game/BluePrints/PlayerWidgets/Telephone/data/S_ChatData` _output_get))))))
        (bind _returnvalue (`KismetArrayLibrary.Array_Add` (`self.CurrentChatMessages`) (`local.LocalMessange`)))
        (set `local.LocalIndex` _returnvalue)
        (if (`.bIsRead_19_95C868AD468D6E59077743BF47C28EC8` (break `/Game/BluePrints/PlayerWidgets/Telephone/data/S_ChatData` _output_get))
          (set `local.CountUnread` "0")
          (else
            (set `local.CountUnread` "1")))
        (set `local.LocalChat` (make `/Game/BluePrints/PlayerWidgets/Telephone/data/S_ChatData` (break `/Game/BluePrints/PlayerWidgets/Telephone/data/S_ChatData` _output_get) (`.ContactName_5_8A672E7F4E0BBF0F0377C289997E0B80` (break `/Game/BluePrints/PlayerWidgets/Telephone/data/S_ChatData` _output_get)) (struct) (`local.CountUnread`) (`self.CurrentChatMessages`)))
        (break)))
    (return (`local.LocalIndex`))
    (else
      (`KismetSystemLibrary.PrintString` "Cообщение не найдено" true true (struct :`R` 1.0 :`B` 0.021061 :`A` 1.0)))))

(fn `GetAllChats`
  (returns (AllChats :type "Array of /Game/BluePrints/PlayerWidgets/Telephone/data/S_ChatData Structure"))
  ; getter
  (return (`self.AllChats`)))

(fn `GetChatByContactID`
  (params (ContactID :type Name))
  (returns (OutChat :type "/Game/BluePrints/PlayerWidgets/Telephone/data/S_ChatData Structure") (bFound :type Boolean) (Index :type Integer))
  (locals (LocalID :type Name) (LocalblsFound :type Boolean :default true) (LocalChatElement :type "/Game/BluePrints/PlayerWidgets/Telephone/data/S_ChatData Structure") (LocalOutChat :type "/Game/BluePrints/PlayerWidgets/Telephone/data/S_ChatData Structure"))
  (set `local.LocalID` ContactID)
  (for (_array_element _array_index) (`self.AllChats`)
    (bind _output_get (set `local.LocalChatElement` _array_element))
    (if (== (break `/Game/BluePrints/PlayerWidgets/Telephone/data/S_ChatData` _output_get) (`local.LocalID`))
      (set `local.LocalblsFound` true)
      (set `local.LocalOutChat` _array_element)
      (break)
      (else
        (set `local.LocalblsFound` false))))
  (return (`local.LocalOutChat`) (`local.LocalblsFound`) _array_index))

(fn `MarkChatAsRead`
  (params (ContactID :type Name))
  (locals (OutChat :type "/Game/BluePrints/PlayerWidgets/Telephone/data/S_ChatData Structure"))
  (bind (_outchat _bfound _index) (`self.GetChatByContactID` ContactID))
  (if _bfound
    (bind _output_get (set `local.OutChat` _outchat))
    (`KismetArrayLibrary.Array_Insert` (`self.AllChats`) (make `/Game/BluePrints/PlayerWidgets/Telephone/data/S_ChatData` (break `/Game/BluePrints/PlayerWidgets/Telephone/data/S_ChatData` _output_get) (`.ContactName_5_8A672E7F4E0BBF0F0377C289997E0B80` (break `/Game/BluePrints/PlayerWidgets/Telephone/data/S_ChatData` _output_get)) (`.LastMessage_12_F2B0695347BFB80FCB242B849E071437` (break `/Game/BluePrints/PlayerWidgets/Telephone/data/S_ChatData` _output_get)) (`.UnreadCount_9_CE92EA344DA6F54D2F2324BEDCB97729` (break `/Game/BluePrints/PlayerWidgets/Telephone/data/S_ChatData` _output_get)) (`.Messages_14_F14D9F5547DC196C2D9B5BA52F908131` (break `/Game/BluePrints/PlayerWidgets/Telephone/data/S_ChatData` _output_get)) true) _index)
    (return)
    (else
      (`KismetSystemLibrary.PrintString` "Hello"))))