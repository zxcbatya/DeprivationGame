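; BP_HouseDoor is an interactable house door that swings open and closed when the player interacts with it.
; OnInteract plays the main door sound at the door's location, then after a short delay flips the IsClosedDoor flag.
; The OpenDoor timeline plays to open and reverses to close, lerping the mesh component's relative yaw between closed and swung-open angles.
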(event `self.OnInteract`
  (params (InteractingPawn :type "Pawn Object Reference"))
  (bind _returnvalue_location (`KismetMathLibrary.BreakTransform` (`self.GetTransform`)))
  ; добавить звуки на двери
  (`GameplayStatics.PlaySoundAtLocation` "/Game/Audio/another/SC_MainDoor.SC_MainDoor" _returnvalue_location (struct) 1.0 1.0 0.0 null null null null)
  (if true
    (`KismetSystemLibrary.Delay` 0.2)
    (bind _output_get (set `self.IsClosedDoor` (`self.IsClosedDoor`)))
    (if _output_get
      (set `self.IsClosedDoor` false)
      (bind (_direction _dooralpha) (`Timeline|OpenDoor` :!label _label)
        (:`Update`
          (bind (_returnvalue_roll _returnvalue_pitch _returnvalue_yaw) (`KismetMathLibrary.BreakRotator` (`KismetMathLibrary.MakeRotator` 0.0 0.0 (`KismetMathLibrary.Lerp` 0.0 -80.0 _dooralpha))))
          (`SceneComponent.K2_SetRelativeRotation` (`self.MeshComponent`) (`KismetMathLibrary.MakeRotator` 0.0 0.0 _returnvalue_yaw) false false)))
      (else
        (set `self.IsClosedDoor` true)
        (goto _label :!via `Reverse`)))))

(fn `UserConstructionScript`)