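; BP_BackPack is a backpack item that sets up its contents on BeginPlay and handles taking vodka or drugs.
; Its item-removed event stores the item and interacting pawn for the consume events.
; Both consume events disable player 0's input during a three-second delay, restore it, then call RemoveItem with the stored pawn.
; Only the drugs path also destroys the stored item actor.
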(event `self.OnItemRemovedFromBackpack`
  (params (Item :type "ItemActor Object Reference") (InteractingPawn :type "Pawn Object Reference"))
  (set `self.CurrentItem` Item)
  (set `self.Interacting PawnRef` InteractingPawn))

(event `self.TakingVodka`
  (`self.DisableInput` (`GameplayStatics.GetPlayerCharacter` 0) (`GameplayStatics.GetPlayerController` 0))
  (`KismetSystemLibrary.Delay` 3.0)
  (`self.EnableInput` (`GameplayStatics.GetPlayerCharacter` 0) (`GameplayStatics.GetPlayerController` 0))
  (`self.RemoveItem` (`self.Interacting PawnRef`)))

(event `self.TakingDrugs`
  (`self.DisableInput` (`GameplayStatics.GetPlayerCharacter` 0) (`GameplayStatics.GetPlayerController` 0))
  (`KismetSystemLibrary.Delay` 3.0)
  (`self.EnableInput` (`GameplayStatics.GetPlayerCharacter` 0) (`GameplayStatics.GetPlayerController` 0))
  (`self.RemoveItem` (`self.Interacting PawnRef`))
  (`self.K2_DestroyActor` (`self.CurrentItem`)))

(event `self.ReceiveBeginPlay`
  (`self.InitializeBackpackContents`))

(fn `UserConstructionScript`)