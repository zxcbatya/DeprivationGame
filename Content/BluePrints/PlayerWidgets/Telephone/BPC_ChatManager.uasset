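; Blueprint component that seeds the in-game telephone chat with its starting contacts and messages.
; On BeginPlay it registers Father and Dima as contacts in the ChatManagerSubsystem, using name and icon color variables plus an initial.
; It then sends two identical placeholder-text messages with Dima's ID as sender and a hard-coded icon asset path.
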(event `self.ReceiveBeginPlay`
  (`ChatManagerSubsystem.CreateContact` (subsystem `ChatManagerSubsystem`) 0 (`self.FatherName`) (`self.FatherIconColor`) "F")
  (`ChatManagerSubsystem.CreateContact` (subsystem `ChatManagerSubsystem`) 1 (`self.DimaName`) (`self.DimaIconColor`) "D")
  (`ChatManagerSubsystem.SendMessage` (subsystem `ChatManagerSubsystem`) 0 "1" "фывфывыфвфывфвфывыфвфывыфв" "DeprivationGame/Content/UI/textures/telephone/user.uasset")
  (`ChatManagerSubsystem.SendMessage` (subsystem `ChatManagerSubsystem`) 0 "1" "фывфывыфвфывфвфывыфвфывыфв" "DeprivationGame/Content/UI/textures/telephone/user.uasset"))