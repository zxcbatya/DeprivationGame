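; Player controller for the menu that opens the main menu widget on BeginPlay.
; It checks a soft class reference to the widget, async-loads the class, then creates the widget, stores a reference and adds it to the viewport.
; If the soft reference is not valid, it prints a Russian warning that no widget is selected, naming the controller.
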(event `self.ReceiveBeginPlay`
  (`parent.ReceiveBeginPlay`)
  (`|ExecutionSequence`
    (:`then_0`
      (`self.Event_OpenWidgetMainMenu` self))))

(event `Event_OpenWidgetMainMenu`
  (if (`KismetSystemLibrary.IsValidSoftClassReference` (`self.MainMenuSoftClassRef`))
    (bind _class (`|LoadAssetClass` (`self.MainMenuSoftClassRef`))
      (:`then`
        (bind _asuser_widget (castclass `UserWidget` _class))
        (bind _returnvalue (`|CreateWidget` _asuser_widget))
        (bind _output_get (set `self.MainMenuWidgetRef` _returnvalue))
        (`UserWidget.AddToViewport` _output_get 0)))
    (else
      (`KismetSystemLibrary.PrintText` (`|FormatText` self "не выбран виджет {self}")))))

(fn `UserConstructionScript`
  (`parent.UserConstructionScript`))