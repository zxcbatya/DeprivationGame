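; Player controller that handles camera look, input mapping contexts, and opening the pause menu and phone UI.
; It adds the player mapping context on BeginPlay, and vehicle interact events add or remove the vehicle context.
; Debug keys P and Tab request soft-class widgets, which return through an event dispatcher to reach the viewport.
; The phone widget is also passed to the character, and CloseWidget removes the widget, resets flags and unpauses.
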(event Custom|EventDis_OpenWidget_Event
  (params (UserWidget :type User%20Widget%20Object%20Reference))
  ;[1 1 1] ивент открытия виджета
  (bind _output_get (Variables|System|SetUser%20Widget UserWidget))
  (if (Variables|System|GetblsOpenGameMenu)
    (UserInterface|Viewport|AddtoViewport _output_get 0)
    (elif (Variables|System|GetblsOpenTelephone)
      (Class|BPICharacter|OpenWidgetTelephone(Message) (Game|GetPlayerCharacter 0) (Variables|System|GetUser%20Widget))
      (UserInterface|Viewport|AddtoViewport (Variables|System|GetUser%20Widget) 0))))

(event Input|EnhancedActionEvents|EnhancedInputActionIA_Loock
  (params (ActionValue :type Vector%202D%20Structure) (ElapsedSeconds :type Float%20%28double-precision%29) (TriggeredSeconds :type Float%20%28double-precision%29) (InputAction :type Input%20Action%20Object%20Reference :default "/Game/BluePrints/Inputs/PayerIput/IA_Loock.IA_Loock"))
  ;[1 1 1] CameraRotate
  (Class|PlayerController|AddYawInput (* (.x ActionValue) (Variables|Default|GetSens)))
  (Class|PlayerController|AddPitchInput (* (.y ActionValue) (Variables|Default|GetSens))))

(event EventBeginPlay
  ;[1 1 1] AddInput
  (Input|SetInputModeGameOnly self false)
  (EventDispatchers|AssignEventDisOpenWidget (delegate Custom|EventDis_OpenWidget_Event))
  (Utilities|FlowControl|Sequence
    (:then_0
      (Input|AddMappingContext (PlayerController|LocalPlayerSubsystems|GetEnhancedInputLocalPlayerSubsystem (Game|GetPlayerController 0)) "/Game/BluePrints/Inputs/PayerIput/IMC_PlayerInput.IMC_PlayerInput" 0 "(bIgnoreAllPressedKeysUntilRelease=True,bForceImmediately=False,bNotifyUserSettings=False)"))))

(event EventExitVehicleInteract
  ;[1 1 1] IMC
  (Input|RemoveMappingContext (PlayerController|LocalPlayerSubsystems|GetEnhancedInputLocalPlayerSubsystem (Game|GetPlayerController 0)) "/Game/BluePrints/VehicleTemplate/Input/Actions/IMC_Vehicle.IMC_Vehicle" "(bIgnoreAllPressedKeysUntilRelease=True,bForceImmediately=False,bNotifyUserSettings=False)"))

(event EventCloseWidget
  (bind _user_widget (Variables|System|GetUser%20Widget))
  ;[1 1 1] close
  (Widget|RemovefromParent _user_widget)
  (CallFunction|SetUIorGameMode false _user_widget)
  (Variables|System|SetblsOpenGameMenu false)
  (Variables|System|SetblsOpenTelephone false)
  (Game|SetGamePaused false))

(event EventEnterVehicleInteract
  ;[1 1 1] IMC
  (Development|PrintString "BIND")
  (Input|AddMappingContext (PlayerController|LocalPlayerSubsystems|GetEnhancedInputLocalPlayerSubsystem (Game|GetPlayerController 0)) "/Game/BluePrints/VehicleTemplate/Input/Actions/IMC_Vehicle.IMC_Vehicle" 0 "(bIgnoreAllPressedKeysUntilRelease=True,bForceImmediately=False,bNotifyUserSettings=False)"))

(event Input|KeyboardEvents|DebugKeyP
  (params (Key :type Key%20Structure :default "None") (ActionValue :type Input%20Action%20Value%20Structure))
  ;[1 1 1] вызов игрового меню
  (:Pressed
    (Utilities|FlowControl|FlipFlop
      (:A
        (CallFunction|EventLoadDataUserWidget (Variables|System|GetPauseMenuSoftClassRef))
        (Development|PrintString "Hello")
        (bind _output_get (Variables|System|SetblsOpenGameMenu true))
        (Game|SetGamePaused _output_get)))))

(event Input|KeyboardEvents|DebugKeyTab
  (params (Key :type Key%20Structure :default "None") (ActionValue :type Input%20Action%20Value%20Structure))
  (:Pressed
    (Utilities|FlowControl|FlipFlop
      (:A
        (CallFunction|EventLoadDataUserWidget (Variables|System|GetPhoneWidgetSoftClassRef))
        (Variables|System|SetblsOpenTelephone true)
        (Input|SetInputModeGameandUI self (Variables|System|GetUser%20Widget) "DoNotLock" true false))
      (:B
        (CallFunction|CloseWidget)))))

(fn ConstructionScript
  (|CallParentFunction))