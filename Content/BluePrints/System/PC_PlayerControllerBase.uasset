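; Base player controller that switches between UI and game input and loads menu widgets on demand.
; SetUIorGameMode toggles input mode and mouse cursor, requiring a valid widget for UI mode but not focusing it.
; Event_LoadDataUserWidget async-loads a soft widget class, creates the widget and broadcasts it through the DisOpenWidget dispatcher, leaving display to listeners.
; An unset class reference prints a Russian-language warning.
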(event `/Game/BluePrints/Interfaces/PlayerController/BPI_PlayerController.SetUI_OrGameMode`
  (params (blsUI_Mode :type Boolean) (FocusUserWidget :type "UserWidget Object Reference"))
  (if blsUI_Mode
    (`/Engine/EditorBlueprintResources/StandardMacros.IsValid` FocusUserWidget
      (:`Is Valid`
        (`WidgetBlueprintLibrary.SetInputMode_UIOnlyEx` self null)
        (set `self.bShowMouseCursor` true)))
    (else
      (`WidgetBlueprintLibrary.SetInputMode_GameOnly` self)
      (set `self.bShowMouseCursor` false))))

(event `Event_LoadDataUserWidget`
  (params (MenuGotoSoftClassRef :type "UserWidget Soft Class Reference"))
  (bind _output_get (set `self.Menu Goto Soft Class Ref` MenuGotoSoftClassRef))
  (if (`KismetSystemLibrary.IsValidSoftClassReference` _output_get)
    (bind _class (`|LoadAssetClass` (`self.Menu Goto Soft Class Ref`))
      (:`Completed`
        (bind _asuser_widget (castclass `UserWidget` _class))
        (bind _returnvalue (`|CreateWidget` _asuser_widget))
        (`/Engine/EditorBlueprintResources/StandardMacros.IsValid` _returnvalue
          (:`Is Valid`
            (`self.EventDis_OpenWidget` _returnvalue)))))
    (else
      (`KismetSystemLibrary.PrintText` (`|FormatText` "не выбран виджет {Self}" self)))))

(fn `UserConstructionScript`)