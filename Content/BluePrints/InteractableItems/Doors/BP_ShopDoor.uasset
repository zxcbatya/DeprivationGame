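; BP_ShopDoor is an interactable shop door that toggles between open and closed on each OnInteract.
; Each interaction plays or reverses the OpenDoor timeline, with IsMoving blocking input until it finishes.
; The timeline sets the Door's yaw from DoorAlpha, which feeds Lerp input A with Alpha fixed at zero, so the raw track value becomes the angle.
; IsFineshed is set on every update.
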(event `self.OnInteract`
  (params (InteractingPawn :type "Pawn Object Reference"))
  (if (not (`self.IsMoving`))
    (set `self.IsMoving` true)
    (bind _output_get (set `self.Opening` (not (`self.Opening`))))
    (if _output_get
      (bind (_direction _dooralpha) (`Timeline|OpenDoor` :!label _label)
        (:`Update`
          (`SceneComponent.K2_SetRelativeRotation` (`self.Door`) (`KismetMathLibrary.MakeRotator` 0.0 0.0 (`KismetMathLibrary.Lerp` _dooralpha 90.0)) false false)
          (set `self.IsFineshed` true))
        (:`Finished`
          (set `self.IsMoving` false)))
      (else
        (goto _label :!via `Reverse`)))))

(fn `UserConstructionScript`)