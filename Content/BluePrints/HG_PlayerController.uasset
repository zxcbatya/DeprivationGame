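; Player controller that handles camera look and switches Enhanced Input mapping contexts for vehicle use.
; The look action feeds yaw and pitch input, scaled by a sensitivity variable.
; BeginPlay adds the player input context, Interact layers the vehicle context on top at equal priority, and ExitVehicle removes only the vehicle context.
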(event `EnhancedInput|/Game/BluePrints/Inputs/PayerIput/IA_Loock`
  (params (ActionValue :type "Vector2D Structure") (ElapsedSeconds :type "Float (double-precision)") (TriggeredSeconds :type "Float (double-precision)") (InputAction :type "InputAction Object Reference" :default "/Game/BluePrints/Inputs/PayerIput/IA_Loock.IA_Loock"))
  ;[1 1 1] CameraRotate
  (:`Triggered`
    (`self.AddYawInput` (* ActionValue_X (`self.Sens`)))
    (`self.AddPitchInput` (* ActionValue_Y (`self.Sens`)))))

(event `self.ReceiveBeginPlay`
  ;[1 1 1] AddInput
  (`EnhancedInputSubsystemInterface.AddMappingContext` (pcsubsystem `EnhancedInputLocalPlayerSubsystem` (`GameplayStatics.GetPlayerController` 0)) "/Game/BluePrints/Inputs/PayerIput/IMC_PlayerInput.IMC_PlayerInput" 0 (struct)))

(event `/Game/BluePrints/Interfaces/BPI_Interaction.Interact`
  (params (InteractorPawn :type "Pawn Object Reference"))
  (`EnhancedInputSubsystemInterface.AddMappingContext` (pcsubsystem `EnhancedInputLocalPlayerSubsystem` (`GameplayStatics.GetPlayerController` 0)) "/Game/BluePrints/Inputs/VehicleInput/IMC_Vehicle.IMC_Vehicle" 0 (struct)))

(event `/Game/BluePrints/Interfaces/BPI_VehicleInteract.ExitVehicle`
  (`EnhancedInputSubsystemInterface.RemoveMappingContext` (pcsubsystem `EnhancedInputLocalPlayerSubsystem` (`GameplayStatics.GetPlayerController` 0)) "/Game/BluePrints/Inputs/VehicleInput/IMC_Vehicle.IMC_Vehicle" (struct)))

(fn `UserConstructionScript`)