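; HUD_Menu is the main menu HUD Blueprint, which sets up the menu screen when play begins.
; BeginPlay switches input to Game and UI, then enables the mouse cursor and click events.
; It points the player's view at a CineCameraActor found in the level, then creates the WPB_MainMenu widget, stores it in MenuRef and adds it to the viewport.
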(event `self.ReceiveBeginPlay`
  (bind _returnvalue (`GameplayStatics.GetPlayerController` 0))
  (`|ExecutionSequence`
    (:`then_0`
      (`WidgetBlueprintLibrary.SetInputMode_GameAndUIEx` (`GameplayStatics.GetPlayerController` 0) null)
      (set `PlayerController.bShowMouseCursor` true _returnvalue)
      (set `PlayerController.bEnableClickEvents` true _returnvalue))
    (:`then_1`
      (bind _returnvalue_2 (`GameplayStatics.GetActorOfClass` "/Script/CinematicCamera.CineCameraActor"))
      (`PlayerController.SetViewTargetWithBlend` _returnvalue _returnvalue_2 0.0 "VTBlend_Linear" 0.0 false))
    (:`then_2`
      (bind _returnvalue_3 (`|CreateWidget` "/Game/BluePrints/Menu/MainMenu/WPB_MainMenu.WPB_MainMenu_C"))
      (bind _output_get (set `self.MenuRef` _returnvalue_3))
      (`UserWidget.AddToViewport` _output_get 0))))

(fn `UserConstructionScript`)