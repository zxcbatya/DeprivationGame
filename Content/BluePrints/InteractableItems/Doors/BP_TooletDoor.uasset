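; BP_TooletDoor is an interactable door that swings open and closed.
; OnInteract prints and toggles the IsClosedDoor flag, then plays or reverses the OpenDoor timeline.
; The timeline's DoorAlpha drives a lerp on the Door component's relative yaw, turning it a quarter turn between closed and open.
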(event `self.OnInteract`
  (params (InteractingPawn :type "Pawn Object Reference"))
  (bind _iscloseddoor (`self.IsClosedDoor`))
  (`KismetSystemLibrary.PrintString` (`KismetStringLibrary.Conv_BoolToString` _iscloseddoor))
  (bind _output_get (set `self.IsClosedDoor` _iscloseddoor))
  (if _output_get
    (set `self.IsClosedDoor` false)
    (bind (_direction _dooralpha) (`Timeline|OpenDoor` :!label _label)
      (:`Update`
        (`SceneComponent.K2_SetRelativeRotation` (`self.Door`) (`KismetMathLibrary.MakeRotator` 0.0 0.0 (`KismetMathLibrary.Lerp` 0.0 -90.0 _dooralpha)) false false)))
    (else
      (set `self.IsClosedDoor` true)
      (goto _label :!via `Reverse`))))

(fn `UserConstructionScript`)